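; Shinbi player base character with automatic ledge hanging, climb-up, drop-down and a montage attack.
; Every tick, forward and downward sphere traces find the wall and ledge height; a ledge near the pelvis socket triggers flying mode and Hang.
; Hang aligns the capsule to the wall and uses the paused climb montage as its pose.
; Input either plays that montage, whose notify moves the capsule forward, or drops; both restore walking.
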(event Custom|Hang
  (bind _w_normal (Variables|Default|GetW_Normal))
  (bind _w_location (Variables|Default|GetW_Location))
  (bind _returnvalue (* _w_normal 45.0))
  (bind _returnvalue_2 (+ _returnvalue _w_location))
  ;[1 1 1] Зависание на препятствии
  (Animation|Montage|PlayMontage (Variables|Character|GetMesh) "/Game/Player/Animation/Shinbi/AM_Hang_to_Crouch.AM_Hang_to_Crouch" 0.0
    (:then
      (Class|AnimInstance|MontagePause (Components|SkeletalMesh|GetAnimInstance (Variables|Character|GetMesh)) "/Game/Player/Animation/Shinbi/AM_Hang_to_Crouch.AM_Hang_to_Crouch")
      (Variables|Default|SetIsClimbing true)
      (Components|MoveComponentTo (Variables|Default|GetCapsuleComponent) (Math|Vector|MakeVector (.x _returnvalue_2) (.y _returnvalue_2) (- (.z (Variables|Default|GetHeight_Loc)) 7e+01)) (Math|Rotator|MakeRotfromX (* _w_normal -1.0)) true true 0.2 false))))

(event Custom|ClimbUp
  (bind _returnvalue (Transformation|GetActorForwardVector))
  ;[1 1 1] Подъем на препятствие
  (Animation|Montage|PlayMontage (Variables|Character|GetMesh) "/Game/Player/Animation/Shinbi/AM_Hang_to_Crouch.AM_Hang_to_Crouch"
    (:OnNotifyBegin
      (Components|MoveComponentTo (Variables|Default|GetCapsuleComponent) (+ (* _returnvalue 1e+02) (Transformation|GetWorldLocation (Variables|Default|GetCapsuleComponent))) (Math|Rotator|MakeRotfromX _returnvalue) true true 0.2 false)
      (Variables|Default|SetIsClimbing false)
      (Pawn|Components|CharacterMovement|SetMovementMode (Variables|Character|GetCharacterMovement) "MOVE_Walking" 0)
      (CallFunction|FinishedClimbing))))

(event Custom|DropDown
  ;[1 1 1] Спуск с препятствия
  (Variables|Default|SetIsClimbing false)
  (Pawn|Components|CharacterMovement|SetMovementMode (Variables|Character|GetCharacterMovement) "MOVE_Walking" 0)
  (Animation|StopAnimMontage "/Game/Player/Animation/Shinbi/AM_Hang_to_Crouch.AM_Hang_to_Crouch"))

(event Custom|FinishedClimbing
  ;[1 1 1] Карабканье на пряпятствие
  (Utilities|FlowControl|DoOnce false) ; enters at Reset
)

(event EventBeginPlay)

(event Collision|EventActorBeginOverlap
  (params (OtherActor :type Actor%20Object%20Reference)))

(event EventTick
  (params (DeltaSeconds :type Float%20%28single-precision%29))
  (CallFunction|ForwardTrace)
  (CallFunction|HeaghtTrace))

(event Input|ActionEvents|InputActionClimdUp
  (params (Key :type Key%20Structure :default "None"))
  ;[1 1 1] Карабканье на пряпятствие
  (:Pressed
    (if (Variables|Default|GetIsClimbing)
      (Utilities|FlowControl|DoOnce false
        (:Completed
          (CallFunction|ClimbUp))))))

(event Input|ActionEvents|InputActionDropDown
  (params (Key :type Key%20Structure :default "None"))
  ;[1 1 1] Карабканье на пряпятствие
  (:Pressed
    (if (Variables|Default|GetIsClimbing)
      (CallFunction|DropDown))))

(event Input|ActionEvents|InputActionAttack
  (params (Key :type Key%20Structure :default "None"))
  (:Pressed
    (Animation|Montage|PlayMontage (Variables|Character|GetMesh) "/Game/Player/Animation/Shinbi/AM_Shinbi_Attack.AM_Shinbi_Attack")))

(fn ConstructionScript)

(fn ForwardTrace
  (bind _returnvalue (Transformation|GetActorLocation))
  (bind _outhit (Collision|SphereTraceByChannel _returnvalue (+ _returnvalue (* (Transformation|GetActorForwardVector) 1.5e+02)) 1e+01 "TraceTypeQuery3" false 0 "ForOneFrame"))
  (Variables|Default|SetW_Normal (.normal _outhit))
  (Variables|Default|SetW_Location (.location _outhit)))

(fn HeaghtTrace
  (bind _returnvalue (Transformation|GetActorLocation))
  (bind _returnvalue_2 (Transformation|GetActorForwardVector))
  (bind _charactermovement (Variables|Character|GetCharacterMovement))
  (bind _returnvalue_3 (* _returnvalue_2 75.0))
  (bind _returnvalue_4 (+ _returnvalue "0, 0,500.000000" _returnvalue_3))
  (bind (_outhit _returnvalue_5) (Collision|SphereTraceByChannel _returnvalue_4 (- _returnvalue_4 "0, 0,500.000000") 1e+01 "TraceTypeQuery3" false 0 "ForOneFrame"))
  (if _returnvalue_5
    (Variables|Default|SetHeight_Loc (.location _outhit))
    (if (Math|Float|InRange(Float) (- (.z (Transformation|GetSocketLocation (Variables|Character|GetMesh) "pelvisSocket")) (.Z (Math|Vector|BreakVector (.location _outhit)))) -5e+01 0.0)
      (if (not (Variables|Default|GetIsClimbing))
        (Pawn|Components|CharacterMovement|SetMovementMode _charactermovement "MOVE_Flying" 0)
        (Components|Movement|StopMovementImmediately _charactermovement)
        (CallFunction|Hang)))))