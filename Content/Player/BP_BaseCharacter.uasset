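; Base player character with vault/climb, directional shield blocking, weapon pickup and an inventory menu toggle.
; Vault & Climb uses line traces to measure wall height and thickness, then plays climb, vault or jump-down montages with collision off.
; A per-tick trace shows the Climb widget near obstacles.
; Timestamped key presses feed an input buffer matched against CommandList, which only flags and prints matches; attack-combo montage logic is unwired.
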(event EventTick
  (params (DeltaSeconds :type Float%20%28single-precision%29))
  (bind _returnvalue (Transformation|GetActorLocation))
  (bind _returnvalue_2 (- _returnvalue "0, 0,44.000000"))
  ;[1 1 1] Widget Climb
  (bind _outactors (Actor|GetAllActorsOfClass "/Game/Enemy/BP_EnemyCharacter.BP_EnemyCharacter_C"))
  (bind _returnvalue_3 (Collision|LineTraceByChannel _returnvalue_2 (+ _returnvalue_2 (* (Transformation|GetActorForwardVector) 7e+01)) "TraceTypeQuery1" false _outactors "None"))
  (if _returnvalue_3
    (Utilities|FlowControl|DoOnce false :!label _label
      (:Completed
        (bind _returnvalue_4 (UserInterface|CreateWidget "/Game/HUD/Climb.Climb_C"))
        (UserInterface|Viewport|AddtoViewport _returnvalue_4 0)))
    (else
      (bind _foundwidgets (Widget|GetAllWidgetsOfClass "/Game/HUD/Climb.Climb_C" true))
      (Widget|RemovefromParent _foundwidgets)
      (goto _label Reset))))

(event Input|ActionEvents|InputActionAttack
  (params (Key :type Key%20Structure :default "None"))
  ;[1 1 1] Attack &ComboAttack
)

(event Input|ActionEvents|InputActionBlocking
  (params (Key :type Key%20Structure :default "None"))
  ;[1 1 1] Blocking
  (:Pressed
    (bind _output_get (Variables|Default|SetIsBlocking true))
    (Variables|Default|SetbUseControllerRotationYaw _output_get)
    (Variables|/Script/Engine.CharacterMovementComponent|SetbOrientRotationToMovement (Variables|Character|GetCharacterMovement) (not _output_get))
    (Variables|Default|SetbCanBeDamaged false))
  (:Released
    (Variables|Default|SetIsBlocking false)))

(event Input|ActionEvents|InputActionEquip
  (params (Key :type Key%20Structure :default "None"))
  (bind _overlappingactors (Collision|GetOverlappingActors "/Game/Weapon/BP_BaseWeapon.BP_BaseWeapon_C" :!class /Script/Engine.Actor))
  (bind _output (Utilities|Array|Get(acopy) _overlappingactors))
  ;[1 1 1] Add Weapon to Inventory
  (:Pressed
    (if (Variables|Default|GetIsOverlappingItem)
      (bind _asbp_base_weapon (Utilities|Casting|CastToBP_BaseWeapon _output))
      (Class|BaszaBaseCharacter|AddtoInventory _asbp_base_weapon)
      (Actor|SetLifeSpan _output 0.0))))

(event Input|ActionEvents|InputActionVault
  (params (Key :type Key%20Structure :default "None"))
  ;[1 1 1] Climbing
  (:Pressed
    (Utilities|Vault&Climb)))

(event Input|ActionEvents|InputActionShowInventoryMenu
  (params (Key :type Key%20Structure :default "None"))
  (:Pressed
    (bind _inventorymenuref (Variables|Inventory|GetInventoryMenuRef)
      (:then
        (Widget|RemovefromParent _inventorymenuref)
        (Variables|Inventory|SetInventoryMenuRef 0)
        (Variables|/Script/Engine.PlayerController|SetbShowMouseCursor (Game|GetPlayerController 0) false))
      (:else
        (bind _returnvalue (UserInterface|CreateWidget "/Game/HUD/InventoryWindow.InventoryWindow_C" (Game|GetPlayerController 0)))
        (bind _output_get (Variables|Inventory|SetInventoryMenuRef _returnvalue))
        (UserInterface|Viewport|AddtoViewport _output_get 0)
        (Variables|/Script/Engine.PlayerController|SetbShowMouseCursor (Game|GetPlayerController 0) true)))))

(event Input|ActionEvents|InputActionAddInputToBuffer
  (params (Key :type Key%20Structure :default "None"))
  (bind _inputbuffer (Variables|Buffer|GetInputBuffer))
  ;[1 1 1] BufferCommand
  (:Pressed
    ;;[1 1 1] CheckBufferCommand
    (for _array_element _inputbuffer
      (if (< (.TimeStamp (Utilities|Struct|BreakFInputInfo _array_element)) (- (Utilities|Time|GetTimeSeconds) 0.2))
        (Utilities|Array|RemoveItem _inputbuffer _array_element)))
    (CallFunction|AddInputtoInputBuffer (Utilities|Struct|MakeFInputInfo (Utilities|String|ToString(Text) (Class|KismetInputLibrary|KeyGetDisplayName Key)) (Utilities|Time|GetTimeSeconds)))))

(fn ConstructionScript)

(fn AttackIsBlocked
  (params (HitActor :type Actor%20Object%20Reference))
  (bind _asbp_base_character (Utilities|Casting|CastToBP_BaseCharacter HitActor)
    (:then
      (return (Math|Boolean|ANDBoolean (< (Math|Vector|DotProduct (Transformation|GetActorForwardVector HitActor) (Transformation|GetActorForwardVector)) -0.5) (Variables|BP_BaseCharacter_C|GetIsBlocking _asbp_base_character) (Variables|Default|GetIsShield))))
    (:CastFailed
      (return false))))

(fn Holster
  (Transformation|AttachComponentToComponent (Variables|Character|GetMesh) "None" "SnapToTarget" "SnapToTarget" "SnapToTarget" true)
  (return))

(fn AddInputtoInputBuffer
  (params (InputInfo :type F%20Input%20Info%20Structure))
  (Utilities|Array|Add (Variables|Buffer|GetInputBuffer) InputInfo)
  (CallFunction|CheckInputBufferforCommand))

(fn CheckInputBufferforCommand
  (bind _inputbuffer (Variables|Buffer|GetInputBuffer))
  (for _array_element (Variables|Buffer|GetCommandList)
    (for _array_element_2 (.Inputs (Utilities|Struct|BreakFCommandInfo _array_element))
      (bind _array_index (Utilities|Array|ForEachLoopwithBreak _inputbuffer :!label _label)
        (:LoopBody
          (if (< (+ _array_index (LocalVariables|GetCorrectSequenceCounter)) (Utilities|Array|Length _inputbuffer))
            (if (Utilities|Enum|Equal(Enum) (.InputName (Utilities|Struct|BreakFInputInfo (Utilities|Array|Get(acopy) (Variables|Buffer|GetInputBuffer) (+ _array_index (LocalVariables|GetCorrectSequenceCounter))))) _array_element_2)
              (bind _result (Math|Integer|IncrementInt (LocalVariables|GetCorrectSequenceCounter))
                (:%20%20
                  (if (== _result (Utilities|Array|Length (.Inputs (Utilities|Struct|BreakFCommandInfo _array_element))))
                    (CallFunction|StartCommand (.Name (Utilities|Struct|BreakFCommandInfo _array_element)))
                    (goto _label Break)
                    (else
                      (goto _label Break)))))
              (else
                (LocalVariables|SetCorrectSequenceCounter 0)))
            (else
              (LocalVariables|SetCorrectSequenceCounter 0))))))))

(fn StartCommand
  (params (CommandName :type String))
  (bind _commandlist (Variables|Buffer|GetCommandList))
  (for (_array_element _array_index) _commandlist
    (if (Utilities|Enum|Equal(Enum) CommandName (.Name (Utilities|Struct|BreakFCommandInfo _array_element)))
      (Utilities|Struct|SetmembersinFCommandInfo (Utilities|Array|Get(acopy) _commandlist _array_index) true)
      (Development|PrintString (.Name (Utilities|Struct|BreakFCommandInfo _array_element)) true true "(R=1.000000,G=0.000000,B=0.179300,A=1.000000)" 5.0))))