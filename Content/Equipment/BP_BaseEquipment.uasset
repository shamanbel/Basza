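; BP_BaseEquipment is a base equipment actor that shows an equip prompt when a BP_BaseCharacter enters its interaction sphere.
; On overlap, if the character's current weapon differs from the sphere's first overlapping weapon, it flags IsOverlappingItem, creates an EquipItemPrompt and calls SetCorrectItemName for the label.
; Leaving the sphere clears the flag and removes every top-level prompt of that class.
; SetCorrectEquipment is an empty stub.
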(event OnComponentBeginOverlap(SphereInteraction)
  (params (OverlappedComponent :type Primitive%20Component%20Object%20Reference) (OtherActor :type Actor%20Object%20Reference) (OtherComp :type Primitive%20Component%20Object%20Reference) (OtherBodyIndex :type Integer) (bFromSweep :type Boolean) (SweepResult :type Hit%20Result%20Structure%20%28by%20ref%29))
  ;[1 1 1] Text to PickupWeapon
  (bind _asbp_base_character (Utilities|Casting|CastToBP_BaseCharacter OtherActor))
  (if (!= (Variables|/Script/Basza.BaszaBaseCharacter|GetCurrentWeapon _asbp_base_character) (Utilities|Array|Get(acopy) (Collision|GetOverlappingActors OverlappedComponent "/Game/Weapon/BP_BaseWeapon.BP_BaseWeapon_C" :!class /Script/Engine.PrimitiveComponent)))
    (Variables|/Script/Basza.BaszaBaseCharacter|SetIsOverlappingItem _asbp_base_character true)
    (bind _returnvalue (UserInterface|CreateWidget "/Game/HUD/EquipItemPrompt.EquipItemPrompt_C"))
    (CallFunction|SetCorrectItemName)
    (UserInterface|Viewport|AddtoViewport _returnvalue 0)))

(event OnComponentEndOverlap(SphereInteraction)
  (params (OverlappedComponent :type Primitive%20Component%20Object%20Reference) (OtherActor :type Actor%20Object%20Reference) (OtherComp :type Primitive%20Component%20Object%20Reference) (OtherBodyIndex :type Integer))
  ;[1 1 1] Text to PickupWeapon
  (bind _asbp_base_character (Utilities|Casting|CastToBP_BaseCharacter OtherActor))
  (Variables|/Script/Basza.BaszaBaseCharacter|SetIsOverlappingItem _asbp_base_character false)
  (bind _foundwidgets (Widget|GetAllWidgetsOfClass "/Game/HUD/EquipItemPrompt.EquipItemPrompt_C" true))
  (for _array_element _foundwidgets
    (Widget|RemovefromParent _array_element)))

(event Custom|SetCorrectItemName
  (params (WidgetRef :type Equip%20Item%20Prompt%20Object%20Reference))
  (Variables|/Game/HUD/EquipItemPrompt.EquipItemPrompt_C|SetItemName WidgetRef (Variables|Default|GetName)))

(event EventBeginPlay)

(event Collision|EventActorBeginOverlap
  (params (OtherActor :type Actor%20Object%20Reference)))

(event EventTick
  (params (DeltaSeconds :type Float%20%28single-precision%29)))

(fn ConstructionScript)

(fn SetCorrectEquipment)