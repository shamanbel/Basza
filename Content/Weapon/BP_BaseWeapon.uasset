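; BP_BaseWeapon is a base weapon actor that the player can pick up and use to damage enemies.
; Its interaction sphere toggles an equip prompt, with SetCorrectItemName left empty here.
; AttachWeapon destroys the character's current weapon and snaps this one to MeleeSocket, while RemoveWeapon only destroys it.
; Collision overlaps during a player attack deal Might-scaled damage, gated by a DoOnce that resets after a delay and clears HasAttack.
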(event OnComponentBeginOverlap(CollisionComponent)
  (params (OverlappedComponent :type Primitive%20Component%20Object%20Reference) (OtherActor :type Actor%20Object%20Reference) (OtherComp :type Primitive%20Component%20Object%20Reference) (OtherBodyIndex :type Integer) (bFromSweep :type Boolean) (SweepResult :type Hit%20Result%20Structure%20%28by%20ref%29))
  ;[1 1 1] Apply damage to enemy
  (bind _asbp_enemy_character (Utilities|Casting|CastToBP_EnemyCharacter OtherActor))
  (bind _asbp_base_character (Utilities|Casting|CastToBP_BaseCharacter (Game|GetPlayerCharacter 0)))
  (if (Variables|/Script/Basza.BaszaBaseCharacter|GetHasAttack _asbp_base_character)
    (Utilities|FlowControl|DoOnce false :!label _label
      (:Completed
        (Class|EnemyCharacter|TakeDamageEnemy _asbp_enemy_character (* (Variables|Default|GetDamageAmount) (Math|Conversions|ToFloat(Integer) (Variables|/Script/Basza.BaszaBaseCharacter|GetMight _asbp_base_character))))
        (Utilities|FlowControl|Delay 1.0)
        (Variables|/Script/Basza.BaszaBaseCharacter|SetHasAttack _asbp_base_character false)
        (goto _label Reset)))))

(event OnComponentBeginOverlap(SphereInteraction)
  (params (OverlappedComponent :type Primitive%20Component%20Object%20Reference) (OtherActor :type Actor%20Object%20Reference) (OtherComp :type Primitive%20Component%20Object%20Reference) (OtherBodyIndex :type Integer) (bFromSweep :type Boolean) (SweepResult :type Hit%20Result%20Structure%20%28by%20ref%29))
  ;[1 1 1] Text to PickupWeapon
  (bind _asbp_base_character (Utilities|Casting|CastToBP_BaseCharacter OtherActor))
  (if (!= (Variables|/Script/Basza.BaszaBaseCharacter|GetCurrentWeapon _asbp_base_character) (Utilities|Array|Get(acopy) (Collision|GetOverlappingActors OverlappedComponent "BP_BaseWeapon_C" :!class /Script/Engine.PrimitiveComponent)))
    (Variables|/Script/Basza.BaszaBaseCharacter|SetIsOverlappingItem _asbp_base_character true)
    (bind _returnvalue (UserInterface|CreateWidget "/Game/HUD/EquipItemPrompt.EquipItemPrompt_C"))
    (CallFunction|SetCorrectItemName _returnvalue)
    (UserInterface|Viewport|AddtoViewport _returnvalue 0)))

(event OnComponentEndOverlap(SphereInteraction)
  (params (OverlappedComponent :type Primitive%20Component%20Object%20Reference) (OtherActor :type Actor%20Object%20Reference) (OtherComp :type Primitive%20Component%20Object%20Reference) (OtherBodyIndex :type Integer))
  ;[1 1 1] Text to PickupWeapon
  (bind _asbp_base_character (Utilities|Casting|CastToBP_BaseCharacter OtherActor))
  (Variables|/Script/Basza.BaszaBaseCharacter|SetIsOverlappingItem _asbp_base_character false)
  (bind _foundwidgets (Widget|GetAllWidgetsOfClass "/Game/HUD/EquipItemPrompt.EquipItemPrompt_C" true))
  (for _array_element _foundwidgets
    (Widget|RemovefromParent _array_element)))

(event Custom|AttachWeapon
  (params (CharacterRef :type BP%20Base%20Character%20Object%20Reference))
  ;[1 1 1] Attach to player
  (bind _currentweapon (Variables|/Script/Basza.BaszaBaseCharacter|GetCurrentWeapon CharacterRef)
    (:then
      (bind _asbp_base_weapon (Utilities|Casting|CastToBP_BaseWeapon _currentweapon))
      (Collision|SetCollisionEnabled (Variables|/Script/Basza.PickUpMaster|GetItemMesh _asbp_base_weapon) "NoCollision")
      (Transformation|DetachFromComponent (Variables|/Script/Basza.PickUpMaster|GetItemMesh _asbp_base_weapon) "KeepRelative" "KeepRelative" "KeepRelative" true)
      (Actor|DestroyActor _currentweapon))
    (:else
      _))
  (Variables|/Script/Basza.BaszaBaseCharacter|SetCurrentWeapon CharacterRef self)
  (Transformation|AttachComponentToComponent (Variables|Default|GetItemMesh) (Variables|/Script/Engine.Character|GetMesh CharacterRef) "MeleeSocket" "SnapToTarget" "KeepRelative" "KeepRelative" true))

(event Custom|RemoveWeapon
  (params (CharacterRef :type BP%20Base%20Character%20Object%20Reference))
  (bind _currentweapon (Variables|/Script/Basza.BaszaBaseCharacter|GetCurrentWeapon CharacterRef)
    (:then
      (bind _asbp_base_weapon (Utilities|Casting|CastToBP_BaseWeapon _currentweapon))
      (Collision|SetCollisionEnabled (Variables|/Script/Basza.PickUpMaster|GetItemMesh _asbp_base_weapon) "NoCollision")
      (Transformation|DetachFromComponent (Variables|/Script/Basza.PickUpMaster|GetItemMesh _asbp_base_weapon) "KeepRelative" "KeepRelative" "KeepRelative" true)
      (Actor|DestroyActor _currentweapon))
    (:else)))

(event EventBeginPlay)

(event EventTick
  (params (DeltaSeconds :type Float%20%28single-precision%29)))

(fn ConstructionScript)

(fn SetCorrectItemName
  (params (WidgetRef :type Equip%20Item%20Prompt%20Object%20Reference)))